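; BP_orc is a side-scrolling orc enemy whose defeat wins the game, flagging the hero's win, playing victory music and opening UI_Menu.
; Tick chases the hero along X and flips the sprite, gated by MoveLock, which the move and attack triggers toggle.
; The attack trigger jumps to an attack animation after a short delay, while capsule overlap deals contact damage.
; Non-lethal hits jump to a hit animation and resume movement.
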(event `self.ReceiveBeginPlay`
  ;[1 1 1] initial
  (bind _asbp_hero (cast `/Game/BluePrints/Character/Hero/BP_hero` (`GameplayStatics.GetPlayerCharacter` 0)))
  (set `self.hero` _asbp_hero))

(event `self.ReceiveTick`
  (params (DeltaSeconds :type "Float (single-precision)"))
  (bind _sprite (`self.Sprite`))
  (bind _returnvalue_x (`KismetMathLibrary.BreakVector` (`SceneComponent.K2_GetComponentLocation` (`self.Sprite`))))
  (bind _returnvalue_x_2 (`KismetMathLibrary.BreakVector` (`SceneComponent.K2_GetComponentLocation` (`Actor.RootComponent` (`self.hero`)))))
  ;[1 1 1] move
  (if (`self.hero_win`)
    (`PrimitiveComponent.SetCollisionEnabled` (`self.CapsuleComponent`) "QueryOnly")
    (elif (not (`self.move_lock`))
      (`/Engine/EditorBlueprintResources/StandardMacros.CompareFloat` _returnvalue_x_2 _returnvalue_x
        (:`>`
          (`self.AddMovementInput` (1.0 0.0 0.0))
          (`SceneComponent.K2_SetRelativeRotation` :`self` _sprite))
        (:`<`
          (`self.AddMovementInput` (-1.0 0.0 0.0))
          (`SceneComponent.K2_SetRelativeRotation` _sprite (struct :`Yaw` 180.0) false false))))))

(event `self.ReceiveAnyDamage`
  (params (Damage :type "Float (single-precision)") (DamageType :type "DamageType Object Reference") (InstigatedBy :type "Controller Object Reference") (DamageCauser :type "Actor Object Reference"))
  (bind _hero_win (`self.hero_win`))
  ;[1 1 1] take damage
  (bind _output_get (set `self.hp` (`KismetMathLibrary.FTrunc` (- (`self.hp`) Damage))))
  (if (> _output_get 0)
    (if (not _hero_win)
      (`PaperZDAnimInstance.JumpToNode` (`PaperZDAnimationComponent.AnimInstance` (`self.AnimationComponent`)) "Jump_hit" "None")
      (set `self.move_lock` false)
      (`GameplayStatics.PlaySound2D` "/Game/Sound/hitAnemy.hitAnemy" 1.0 1.0 0.0 null null))
    (elif (not _hero_win)
      (set `self.hero_win` true)
      (`GameplayStatics.PlaySound2D` "/Game/music/super_mario_win.super_mario_win" 1.0 1.0 0.0 null null)
      (set `/Game/BluePrints/Character/Hero/BP_hero.Win` true (`self.hero`))
      (bind _returnvalue (`|CreateWidget` "/Game/BluePrints/Character/UI/UI_Menu.UI_Menu_C" (`GameplayStatics.GetPlayerController` 0)))
      (`UserWidget.AddToViewport` _returnvalue 0))))

(event `self.CapsuleComponent.OnComponentBeginOverlap`
  (params (OverlappedComponent :type "PrimitiveComponent Object Reference") (OtherActor :type "Actor Object Reference") (OtherComp :type "PrimitiveComponent Object Reference") (OtherBodyIndex :type Integer) (bFromSweep :type Boolean) (SweepResult :type "HitResult Structure (by ref)"))
  (bind _returnvalue (`self.GetOwner`))
  (bind _returnvalue_x (`KismetMathLibrary.BreakVector` (`SceneComponent.K2_GetComponentLocation` (`self.Sprite`))))
  ;[1 1 1] body damage
  (`/Engine/EditorBlueprintResources/StandardMacros.IsValid` _returnvalue
    (:`Is Valid`
      (if (== OtherActor _returnvalue)
        _
        (elif (> (`self.hp`) 0)
          (bind _asbp_hero (cast `/Game/BluePrints/Character/Hero/BP_hero` OtherActor))
          (`GameplayStatics.ApplyDamage` _asbp_hero 1.0)
          (set `/Game/BluePrints/Character/Hero/BP_hero.DmgX` _returnvalue_x (`self.hero`)))))))

(event `self.AtackTriger.OnComponentBeginOverlap`
  (params (OverlappedComponent :type "PrimitiveComponent Object Reference") (OtherActor :type "Actor Object Reference") (OtherComp :type "PrimitiveComponent Object Reference") (OtherBodyIndex :type Integer) (bFromSweep :type Boolean) (SweepResult :type "HitResult Structure (by ref)"))
  (bind _hero (`self.hero`))
  (bind _returnvalue_x (`KismetMathLibrary.BreakVector` (`SceneComponent.K2_GetComponentLocation` (`self.Sprite`))))
  ;[1 1 1] atack
  (if (`self.hero_win`)
    _
    (elif (== (`/Game/BluePrints/Character/Hero/BP_hero.hp` _hero) 0.0)
      _
      (elif (== _hero OtherActor)
        (`KismetSystemLibrary.Delay` 0.25)
        (set `/Game/BluePrints/Character/Hero/BP_hero.DmgX` _returnvalue_x (`self.hero`))
        (`PaperZDAnimInstance.JumpToNode` (`PaperZDAnimationComponent.AnimInstance` (`self.AnimationComponent`)) "Jump_atack" "None")
        (set `self.atack` true)
        (set `self.move_lock` true)))))

(event `self.AtackTriger.OnComponentEndOverlap`
  (params (OverlappedComponent :type "PrimitiveComponent Object Reference") (OtherActor :type "Actor Object Reference") (OtherComp :type "PrimitiveComponent Object Reference") (OtherBodyIndex :type Integer))
  ;[1 1 1] atack
  (if (== (`self.hero`) OtherActor)
    (set `self.atack` false)
    (set `self.move_lock` false)))

(event `self.MoveTrigger.OnComponentBeginOverlap`
  (params (OverlappedComponent :type "PrimitiveComponent Object Reference") (OtherActor :type "Actor Object Reference") (OtherComp :type "PrimitiveComponent Object Reference") (OtherBodyIndex :type Integer) (bFromSweep :type Boolean) (SweepResult :type "HitResult Structure (by ref)"))
  ;[1 1 1] Преследование
  (if (== OtherActor (`self.hero`))
    (set `self.move_lock` false)))

(event `self.MoveTrigger.OnComponentEndOverlap`
  (params (OverlappedComponent :type "PrimitiveComponent Object Reference") (OtherActor :type "Actor Object Reference") (OtherComp :type "PrimitiveComponent Object Reference") (OtherBodyIndex :type Integer))
  ;[1 1 1] Преследование
  (if (== OtherActor (`self.hero`))
    (set `self.move_lock` true)
    (set `self.atack` false)))

(fn `UserConstructionScript`)