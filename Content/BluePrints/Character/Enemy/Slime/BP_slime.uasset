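; BP_slime is a 2D slime enemy that patrols along the X axis, flipping its sprite to face its heading.
; BoxHit overlaps reverse its direction, except with the hero, who takes damage while the slime keeps its heading and briefly pauses.
; When damaged, it is knocked away from the hero and briefly stunned.
; At zero HP it plays a death animation, randomly drops a coin, apple or nothing, then destroys itself.
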(event `self.ReceiveBeginPlay`
  ;[1 1 1] Comment
  (bind _asbp_hero (cast `/Game/BluePrints/Character/Hero/BP_hero` (`GameplayStatics.GetPlayerCharacter` 0)))
  (set `self.hero` _asbp_hero))

(event `self.ReceiveTick`
  (params (DeltaSeconds :type "Float (single-precision)"))
  (bind _sprite (`self.Sprite`))
  ;[1 1 1] Comment
  (if (`self.Stop`)
    _
    (elif (`self.swapVector`)
      (`self.AddMovementInput` (1.0 0.0 0.0) -1.0)
      (`SceneComponent.K2_SetWorldRotation` _sprite (struct :`Yaw` 180.0) false false)
      (else
        (`self.AddMovementInput` (1.0 0.0 0.0))
        (`SceneComponent.K2_SetWorldRotation` :`self` _sprite)))))

(event `self.BoxHit.OnComponentBeginOverlap`
  (params (OverlappedComponent :type "PrimitiveComponent Object Reference") (OtherActor :type "Actor Object Reference") (OtherComp :type "PrimitiveComponent Object Reference") (OtherBodyIndex :type Integer) (bFromSweep :type Boolean) (SweepResult :type "HitResult Structure (by ref)"))
  (bind _returnvalue (`self.GetOwner`))
  (bind _charactermovement (`self.CharacterMovement`))
  (bind _returnvalue_x (`KismetMathLibrary.BreakVector` (`SceneComponent.K2_GetComponentLocation` (`self.Sprite`))))
  ;[1 1 1] Comment
  (`/Engine/EditorBlueprintResources/StandardMacros.IsValid` _returnvalue
    (:`Is Valid`
      (if (not (== _returnvalue OtherActor))
        (set `/Game/BluePrints/Character/Hero/BP_hero.DmgX` _returnvalue_x (`self.hero`))
        (set `self.swapVector` (not (`self.swapVector`)))
        (bind _asbp_hero (cast `/Game/BluePrints/Character/Hero/BP_hero` OtherActor))
        (`GameplayStatics.ApplyDamage` _asbp_hero 1.0)
        (set `self.swapVector` (not (`self.swapVector`)))
        (`CharacterMovementComponent.SetMovementMode` _charactermovement "MOVE_None" 0)
        (`KismetSystemLibrary.Delay` 0.5)
        (`CharacterMovementComponent.SetMovementMode` _charactermovement "MOVE_Walking" 0)))))

(event `self.ReceiveAnyDamage`
  (params (Damage :type "Float (single-precision)") (DamageType :type "DamageType Object Reference") (InstigatedBy :type "Controller Object Reference") (DamageCauser :type "Actor Object Reference"))
  (bind _returnvalue (`self.K2_GetActorLocation`))
  (bind _hp (`self.hp`))
  (bind _returnvalue_x (`KismetMathLibrary.BreakVector` (`SceneComponent.K2_GetComponentLocation` (`self.Sprite`))))
  (bind _returnvalue_x_2 (`KismetMathLibrary.BreakVector` (`SceneComponent.K2_GetComponentLocation` (`Actor.RootComponent` (`self.hero`)))))
  ;[1 1 1] Comment
  (set `self.hp` (`KismetMathLibrary.FTrunc` (- _hp Damage)))
  (`GameplayStatics.PlaySound2D` "/Game/Sound/hitAnemy.hitAnemy" 1.0 1.0 0.0 null null)
  (if (> _hp 0)
    (`/Engine/EditorBlueprintResources/StandardMacros.CompareFloat` _returnvalue_x _returnvalue_x_2
      (:`>`
        (`self.LaunchCharacter` (200.0 0.0 100.0) true true))
      (:`<`
        (`self.LaunchCharacter` (-200.0 0.0 100.0) true true)))
    (`PaperZDAnimInstance.JumpToNode` (`PaperZDAnimationComponent.AnimInstance` (`self.AnimationComponent`)) "hitJump" "None")
    (set `self.Stop` true)
    (`KismetSystemLibrary.Delay` 0.5)
    (set `self.Stop` false)
    (else
      (`PaperZDAnimInstance.JumpToNode` (`PaperZDAnimationComponent.AnimInstance` (`self.AnimationComponent`)) "isDead" "None")
      (`PrimitiveComponent.SetCollisionEnabled` (`self.BoxHit`) "NoCollision")
      (set `self.Stop` true)
      (`KismetSystemLibrary.Delay` 0.5)
      (switch `int` (`KismetMathLibrary.RandomInteger` 5)
        (:`Default`
          _)
        (:`0`
          (`|SpawnActorFromClass` "/Game/BluePrints/item/coin/drop_coin.drop_coin_C" (`KismetMathLibrary.MakeTransform` _returnvalue) "Undefined" "MultiplyWithRoot" null null))
        (:`1`
          (`|SpawnActorFromClass` "/Game/BluePrints/item/fruit/apple.apple_C" (`KismetMathLibrary.MakeTransform` _returnvalue) "Undefined" "MultiplyWithRoot" null null)))
      (`self.K2_DestroyActor`))))

(fn `UserConstructionScript`)